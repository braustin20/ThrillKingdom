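; BPPawnTest is a test player pawn that acts as a free-moving camera with planar movement and stepped zoom.
; Forward and Right axis input move it by MoveSpeed along its flattened forward vector and its right vector, without sweeping or frame-time scaling.
; ZoomIn and ZoomOut shift it by ZoomFactor along a diagonal of up plus horizontal backward.
; Zooming in only works while its height is above 10 units.
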(event `InputAxis|Forward`
  (params (AxisValue :type "Float (single-precision)"))
  (`self.K2_SetActorLocation` (+ (`self.K2_GetActorLocation`) (* (`KismetMathLibrary.MakeVector` (.x (`self.GetActorForwardVector`)) (.y (`self.GetActorForwardVector`))) (* (`self.MoveSpeed`) AxisValue)))))

(event `InputAction|ZoomIn`
  (:`Pressed`
    (if (> (.z (`self.K2_GetActorLocation`)) 10.0)
      (`self.K2_SetActorLocation` (+ (* (+ (`self.GetActorUpVector`) (`KismetMathLibrary.MakeVector` (.x (* (`self.GetActorForwardVector`) -1.0)) (.y (* (`self.GetActorForwardVector`) -1.0)))) (* (`self.ZoomFactor`) -1.0)) (`self.K2_GetActorLocation`))))))

(event `InputAxis|Right`
  (params (AxisValue :type "Float (single-precision)"))
  (`self.K2_SetActorLocation` (+ (`self.K2_GetActorLocation`) (* (`self.GetActorRightVector`) (* (`self.MoveSpeed`) AxisValue)))))

(event `InputAction|ZoomOut`
  (:`Pressed`
    (`self.K2_SetActorLocation` (+ (* (+ (`self.GetActorUpVector`) (`KismetMathLibrary.MakeVector` (.x (* (`self.GetActorForwardVector`) -1.0)) (.y (* (`self.GetActorForwardVector`) -1.0)))) (`self.ZoomFactor`)) (`self.K2_GetActorLocation`)))))

(fn `UserConstructionScript`)