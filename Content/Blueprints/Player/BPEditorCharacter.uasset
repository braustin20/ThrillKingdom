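; BPEditorCharacter is a player-controlled character with movement and zoom input, named for use in an editor.
; Forward and Right axes feed movement input along the actor's own vectors, with the forward vector's Z zeroed so looking up or down adds no vertical movement.
; ZoomIn and ZoomOut presses multiply the actor's location by their factors without sweep, so zoom scales its position relative to the world origin.
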(event `InputAxis|Forward`
  (params (AxisValue :type "Float (single-precision)"))
  (`self.AddMovementInput` (`KismetMathLibrary.MakeVector` (.x (`self.GetActorForwardVector`)) (.y (`self.GetActorForwardVector`))) AxisValue))

(event `InputAction|ZoomIn`
  (:`Pressed`
    (`self.K2_SetActorLocation` (* (`self.K2_GetActorLocation`) (`self.ZoomInFactor`)))))

(event `InputAxis|Right`
  (params (AxisValue :type "Float (single-precision)"))
  (`self.AddMovementInput` (`self.GetActorRightVector`) AxisValue))

(event `InputAction|ZoomOut`
  (:`Pressed`
    (`self.K2_SetActorLocation` (* (`self.K2_GetActorLocation`) (`self.ZoomOutFactor`)))))

(fn `UserConstructionScript`)